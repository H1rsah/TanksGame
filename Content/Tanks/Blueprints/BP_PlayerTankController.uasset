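; Player controller for the tank game that shows the in-game HUD and toggles the main menu.
; On BeginPlay it casts the HUD to MyHUD, stores it and shows the in-game widget.
; The M key drives a FlipFlop that swaps between the main menu and in-game widgets, freezing and resuming the game through global time dilation rather than pausing it.
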(event EventBeginPlay
  (bind _asmy_hud (Utilities|Casting|CastToMyHUD (HUD|GetHUD)))
  (bind _output_get (Variables|Default|SetHUD _asmy_hud))
  (Class|MyHUD|ShowWidget _output_get "Wid_InGame"))

(event Input|KeyboardEvents|M
  (params (Key :type Key%20Structure :default "None"))
  (bind _hud (Variables|Default|GetHUD))
  (:Pressed
    (Utilities|FlowControl|FlipFlop
      (:A
        (Class|MyHUD|ShowWidget _hud "Wid_MainMenu")
        (Utilities|Time|SetGlobalTimeDilation 0.0))
      (:B
        (Class|MyHUD|ShowWidget _hud "Wid_InGame")
        (Utilities|Time|SetGlobalTimeDilation 1.0)))))

(fn ConstructionScript)